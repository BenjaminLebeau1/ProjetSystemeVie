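; BP_PlayerState is the player state that keeps the player's health in BP_GameInstance through its AC_Health component.
; On BeginPlay it restores saved health from the game instance, or resets it the first time and sets an initialized flag.
; Each health change writes current and max values back to the game instance.
; On death it asks BP_ThirdPersonGameMode to start respawning player controller 0.
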(event OnHealthChange(AC_Health)
  (params (CurrentHealth :type Float%20%28double-precision%29) (MaxHealth :type Float%20%28double-precision%29))
  (CallFunction|SaveCurrentHealth CurrentHealth)
  (CallFunction|SaveMaxHealth MaxHealth))

(event OnDeath(AC_Health)
  (bind _asbp_third_person_game_mode (Utilities|Casting|CastToBP_ThirdPersonGameMode (Game|GetGameMode)))
  (Default|StartRespawn _asbp_third_person_game_mode (Game|GetPlayerController 0)))

(event EventTick
  (params (DeltaSeconds :type Float%20%28single-precision%29)))

(event EventBeginPlay
  (bind _asbp_game_instance (Utilities|Casting|CastToBP_GameInstance (Game|GetGameInstance)))
  (bind _output_get (Variables|Default|SetRef_GameInstence _asbp_game_instance))
  (if (Variables|/Game/Game/Blueprints/BP_GameInstance.BP_GameInstance_C|GetHealthInitialized_Gl _output_get)
    (CallFunction|LoadHealthfromGameInstence)
    (else
      (Default|ResetHealth (Variables|Default|GetAC_Health))
      (Variables|/Game/Game/Blueprints/BP_GameInstance.BP_GameInstance_C|SetHealthInitialized_Gl (Variables|Default|GetRef_GameInstence) true))))

(fn ConstructionScript)

(fn SaveCurrentHealth
  (params (NewHealth :type Float%20%28double-precision%29))
  (Variables|/Game/Game/Blueprints/BP_GameInstance.BP_GameInstance_C|SetCurrentHealth_Gl (Variables|Default|GetRef_GameInstence) NewHealth))

(fn SaveMaxHealth
  (params (NewMaxHealth :type Float%20%28double-precision%29))
  (Variables|/Game/Game/Blueprints/BP_GameInstance.BP_GameInstance_C|SetmaxHealth_Gl (Variables|Default|GetRef_GameInstence) NewMaxHealth))

(fn LoadHealthfromGameInstence
  (bind _output_get (Variables|/Game/Game/Blueprints/Components/AC_Health.AC_Health_C|SetMaxHealth (Variables|Default|GetAC_Health) (Variables|/Game/Game/Blueprints/BP_GameInstance.BP_GameInstance_C|GetmaxHealth_Gl (Variables|Default|GetRef_GameInstence))))
  (bind _output_get_2 (Variables|/Game/Game/Blueprints/Components/AC_Health.AC_Health_C|SetCurrentHealth (Variables|Default|GetAC_Health) (Variables|/Game/Game/Blueprints/BP_GameInstance.BP_GameInstance_C|GetCurrentHealth_Gl (Variables|Default|GetRef_GameInstence))))
  (Default|CallOnHealthChange (Variables|Default|GetAC_Health) _output_get_2 _output_get))